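; Final door actor that slides open when the player pawn overlaps it and no crystals are left.
; On overlap it stores both leaves' starting world X positions and plays a timeline.
; Each timeline update offsets the left and right doors in opposite directions along world X.
; A flag set when the timeline finishes keeps the door from opening again.
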(event Collision|EventActorBeginOverlap
  (params (OtherActor :type Actor%20Object%20Reference))
  (Utilities|IsPlayerPawn OtherActor
    (:IsPlayerPawn
      (Utilities|AnyCrystalsLeft
        (:NoCrystals
          (if (not (Variables|Default|GetdoorAlreadyOpen))
            ;[1 1 1] Obtener posicion inicial de las puertas.
            (Variables|Default|SetleftDoorXPos (.x (Transformation|GetWorldLocation (Variables|Default|GetLeftDoor))))
            (Variables|Default|SetrightDoorXPos (.x (Transformation|GetWorldLocation (Variables|Default|GetRightDoor))))
            (bind _newtrack_0 (Timeline|OpenDoorsTimeline PlayFromStart)
              (:Update
                ;[1 1 1] Hacer en cada update el movimiento relativo de la puerta.
                (CallFunction|ReallocateLeftDoor _newtrack_0)
                (CallFunction|ReallocateRightDoor _newtrack_0))
              (:Finished
                (Variables|Default|SetdoorAlreadyOpen true)))))))))

(event EventBeginPlay
  (Variables|Default|SetdoorAlreadyOpen false))

(fn ConstructionScript)

(fn ReallocateLeftDoor
  (params (B :type Float%20%28single-precision%29))
  (bind _leftdoor (Variables|Default|GetLeftDoor))
  (bind _returnvalue (Transformation|GetWorldLocation _leftdoor))
  (Transformation|SetWorldLocation _leftdoor (Math|Vector|MakeVector (- (Variables|Default|GetleftDoorXPos) B) (.y _returnvalue) (.z _returnvalue)) false false))

(fn ReallocateRightDoor
  (params (B :type Float%20%28single-precision%29))
  (bind _rightdoor (Variables|Default|GetRightDoor))
  (bind _returnvalue (Transformation|GetWorldLocation _rightdoor))
  (Transformation|SetWorldLocation _rightdoor (Math|Vector|MakeVector (+ (Variables|Default|GetrightDoorXPos) B) (.y _returnvalue) (.z _returnvalue)) false false))