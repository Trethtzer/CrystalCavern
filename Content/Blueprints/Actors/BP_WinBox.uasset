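; BP_WinBox is a level-exit trigger actor that advances the game when the player overlaps it with every crystal collected.
; On overlap it passes the other actor through an IsPlayer check, then confirms no Crystal actors remain in the world.
; It finds the current level by name in its LevelNames array and opens the following entry, or quits the game on the last level.
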(event Collision|EventActorBeginOverlap
  (params (OtherActor :type Actor%20Object%20Reference))
  (Utilities|IsPlayer OtherActor
    (:Is%20player%20paaawn
      ;[1 1 1] Continue if crystals collected
      (if (not (CallFunction|CrystalsRemaining))
        (if (CallFunction|IsLastLevel)
          ;[1 1 1] Quits the game
          (Game|QuitGame (Game|GetPlayerController 0) "Quit" false)
          (else
            ;[1 1 1] Opens next level
            (Utilities|OpenLevel (Utilities|Array|Get(acopy) (Variables|Default|GetlevelNames) (+ (CallFunction|GetCurrentLevelIndex) 1)))))))))

(fn ConstructionScript)

(fn CrystalsRemaining
  (bind _outactors (Actor|GetAllActorsOfClass "/Game/Blueprints/Actors/Crystal.Crystal_C"))
  (return (> (Utilities|Array|Length _outactors) 0)))

(fn GetCurrentLevelIndex
  (bind _returnvalue (Game|GetCurrentLevelName true))
  (return (Utilities|Array|FindItem (Variables|Default|GetlevelNames) _returnvalue)))

(fn IsLastLevel
  (return (== (CallFunction|GetCurrentLevelIndex) (Utilities|Array|LastIndex (Variables|Default|GetlevelNames)))))